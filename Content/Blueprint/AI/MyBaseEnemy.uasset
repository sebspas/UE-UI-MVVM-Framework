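; Base enemy character Blueprint that shows a health bar and handles its own death for AI-controlled enemies.
; On BeginPlay it caches the HealthBar from its widget component and refreshes it whenever the Health component reports a change.
; On death it ragdolls the mesh from the pelvis down the bone chain, disables tick and capsule collision, removes the widget and stops the AI controller's brain logic.
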(event `self.ReceiveBeginPlay`
  (bind _health (`self.Health`))
  ;[1 1 1] HealthBar
  (bind _ashealth_bar (cast `/Game/UI/HealthBar` (`WidgetComponent.GetWidget` (`self.Widget`))))
  (bind _output_get (set `self.Ref_enemyHealthBar` _ashealth_bar))
  (`/Game/UI/HealthBar.UpdateHealth` _output_get (`Health.Current` _health) (`Health.MaxHealth` _health)))

(event `self.Health.HealthChanged`
  (params (Current :type "Float (single-precision)") (Max :type "Float (single-precision)"))
  ;[1 1 1] HealthBar
  (`/Game/UI/HealthBar.UpdateHealth` (`self.Ref_enemyHealthBar`) Current Max))

(event `self.Health.Death`
  (bind _mesh (`self.Mesh`))
  ;[1 1 1] OnDeath
  (`SkeletalMeshComponent.SetAllBodiesBelowSimulatePhysics` _mesh "pelvis" true true)
  (`SkeletalMeshComponent.SetAllBodiesBelowPhysicsBlendWeight` _mesh "pelvis" 1.0 false true)
  (`self.SetActorTickEnabled` false)
  (`PrimitiveComponent.SetCollisionEnabled` (`self.CapsuleComponent`) "NoCollision")
  (`ActorComponent.K2_DestroyComponent` (`self.Widget`))
  (`BrainComponent.StopLogic` (`AIController.BrainComponent` (`AIBlueprintHelperLibrary.GetAIController` self)) ""))

(fn `UserConstructionScript`)