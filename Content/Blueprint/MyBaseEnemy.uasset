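; Base enemy Blueprint that chases the player character and attacks it in melee.
; When PawnSensing sees a TopDownCharacter, it stores that pawn as the target and moves toward it with AIMoveTo.
; On arrival it raises a SwordSlash flag, waits briefly, damages the target's Health component without rechecking range, then clears the flag and resumes the chase in a loop.
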(event `self.PawnSensing.OnSeePawn`
  (params (Pawn :type "Pawn Object Reference"))
  (if (not (`self.SwordSlash`))
    (bind _astop_down_character (cast `/Game/Blueprint/TopDownCharacter` Pawn))
    (set `self.PlayerTarget` _astop_down_character)
    (`|AIMoveTo` self (0.0 0.0 0.0) (`self.PlayerTarget`) :!label _label
      (:`OnSuccess`
        (set `self.SwordSlash` true)
        (`KismetSystemLibrary.Delay` 1.0)
        (`Health.ApplyHealthChange` (`/Game/Blueprint/TopDownCharacter.Health` (`self.PlayerTarget`)) -10.0)
        (set `self.SwordSlash` false)
        (goto _label)))))

(fn `UserConstructionScript`)