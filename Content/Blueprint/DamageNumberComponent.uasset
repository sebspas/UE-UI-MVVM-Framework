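; Actor component that shows floating damage numbers for its owner as DamageNumber widgets.
; AddDamageNumber creates a widget tied to the owning actor, tracks it in DamageWidgets, initializes it with the damage value and a one-second lifetime, and adds it to the viewport.
; RemoveDamageNumber takes a widget, pulls it from the viewport, hides it and drops it from the tracked list.
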(fn `AddDamageNumber`
  (params (NewDamage :type "Float (double-precision)"))
  (bind _returnvalue (`|CreateWidget` "/Game/UI/DamageNumber.DamageNumber_C"))
  (set `/Game/UI/DamageNumber.ActorOwner` (`self.GetOwner`) _returnvalue)
  (`KismetArrayLibrary.Array_Add` (`self.DamageWidgets`) _returnvalue)
  (`/Game/UI/DamageNumber.Init` _returnvalue NewDamage self 1.0)
  (`UserWidget.AddToViewport` _returnvalue 0))

(fn `RemoveDamageNumber`
  (params (Index :type "/Game/UI/DamageNumber Object Reference"))
  (`Widget.RemoveFromParent` Index)
  (`Widget.SetVisibility` Index "Hidden")
  (`KismetArrayLibrary.Array_RemoveItem` (`self.DamageWidgets`) Index))