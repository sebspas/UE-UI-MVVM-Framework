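; Actor component that shows its owner as a point of interest on the player's HUD minimap.
; On BeginPlay, after a short delay for the minimap to be ready, it binds OnDeath to the OnOwnerDeath event.
; It then gets the minimap from the TopDownCharacter's HUD, caches it and adds the owner as a POI.
; OnDeath removes that POI from the cached minimap.
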(event `self.ReceiveBeginPlay`
  ;[1 1 1] Create Widget on map
  (`KismetSystemLibrary.Delay` 0.2) ; delay needed to wait for minimap to be ready
  (add `self.OnOwnerDeath` (delegate `OnDeath`))
  (bind _astop_down_character (cast `/Game/Blueprint/Player/TopDownCharacter` (`GameplayStatics.GetPlayerCharacter` 0)))
  (bind _output_get (set `self.Minimap` (`/Game/UI/HUD_Player.Minimap` (`/Game/Blueprint/Player/TopDownCharacter.Player_HUD` _astop_down_character))))
  (`/Game/UI/Minimap/Minimap.AddPOI` _output_get (`self.GetOwner`)))

(event `OnDeath`
  ;[1 1 1] OnDeath
  (`/Game/UI/Minimap/Minimap.RemovePOI` (`self.Minimap`) (`self.GetOwner`)))